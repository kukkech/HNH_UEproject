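; BP_ChikenPatrolFix is a chicken pawn that endlessly walks a fixed patrol route.
; On BeginPlay it starts a looping animation on its skeletal mesh, then chains AI MoveTo calls through the first four PatrolPath1 points.
; The last successful move loops back to the first point; failed moves have no handling, so the patrol stops there.
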(event `self.ReceiveBeginPlay`
  (bind _patrolpath_1 (`self.PatrolPath_1`))
  (`|ExecutionSequence`
    (:`then_0`
      (`SkeletalMeshComponent.PlayAnimation` (`self.SK_Chiken`) "/Game/HNH_Project/ImportedFbx/Anim/Anim_Action.Anim_Action" true))
    (:`then_1`
      (`|AIMoveTo` self (`|GetArrayItem` _patrolpath_1) null :!label _label
        (:`OnSuccess`
          (`|AIMoveTo` self (`|GetArrayItem` _patrolpath_1 1) null
            (:`OnSuccess`
              (`|AIMoveTo` self (`|GetArrayItem` _patrolpath_1 2) null
                (:`OnSuccess`
                  (`|AIMoveTo` self (`|GetArrayItem` _patrolpath_1 3) null
                    (:`OnSuccess`
                      (goto _label))))))))))))

(fn `UserConstructionScript`)