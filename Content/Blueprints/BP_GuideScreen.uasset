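; BP_GuideScreen is a guide screen that reveals text on a text render component with a typewriter effect.
; On BeginPlay, a looping timer at TypeSpeed appends one character of InputText per tick to the displayed string.
; When the string completes, it clears the timer, waits briefly, then restarts typing with a hardcoded "part 2" message, which then repeats indefinitely.
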(event `self.ReceiveBeginPlay`
  (`self.Type text`))

(event `Type text`
  (bind _returnvalue (`KismetSystemLibrary.K2_SetTimerDelegate` (delegate `Set Text`) (`self.Type Speed`) true)))

(event `Set Text`
  (bind _output_get (set `self.Displayed Text` (`KismetStringLibrary.Concat_StrStr` (`self.Displayed Text`) (`|GetArrayItem` (`KismetStringLibrary.GetCharacterArrayFromString` (`self.Input Text`)) (`self.Index`)))))
  ;[1 1 1] Comment
  (`TextRenderComponent.K2_SetText` (`self.TextRender`) (`KismetTextLibrary.Conv_StringToText` _output_get))
  (bind _result (`/Engine/EditorBlueprintResources/StandardMacros.IncrementInt` (`self.Index`))
    (:`  `
      (if (== _result (`KismetArrayLibrary.Array_Length` (`KismetStringLibrary.GetCharacterArrayFromString` (`self.Input Text`))))
        (`KismetSystemLibrary.K2_ClearAndInvalidateTimerHandle` (stale `Type text` _returnvalue))
        (`KismetSystemLibrary.Delay` 1.0)
        (set `self.Input Text` "This is part 2")
        (set `self.Displayed Text` "")
        (set `self.Index` 0)
        (`self.Type text`)))))

(fn `UserConstructionScript`)